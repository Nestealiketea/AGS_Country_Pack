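; Game mode for the VigilanteMovement shared content that chooses which pawn class players spawn as and handles respawning.
; The default pawn class lookup returns a settable movement pawn class when valid, otherwise falls back to the parent's choice.
; A Respawn event destroys the controller's current pawn and restarts the player, so the new pawn uses that class selection.
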(event `Respawn`
  (params (Controller :type "Controller Object Reference"))
  (`self.K2_DestroyActor` (`Controller.K2_GetPawn` Controller))
  (`self.RestartPlayer` Controller))

(fn `GetDefaultPawnClassForController`
  (params (InController :type "Controller Object Reference"))
  (returns (ReturnValue :type "Object Class Reference"))
  (bind _movementpawnclass (`self.MovementPawnClass`))
  (bind _returnvalue (`parent.GetDefaultPawnClassForController` InController))
  (return (select `bool` (`KismetSystemLibrary.IsValidClass` _movementpawnclass) :`false` _returnvalue :`true` _movementpawnclass :!type "Object Class Reference")))

(fn `SetMovementPawnClass`
  (params (MovementPawnClass :type "Pawn Class Reference"))
  (set `self.MovementPawnClass` MovementPawnClass))

(fn `UserConstructionScript`)