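; Component on a BP_BaseVehicle that supplies the data for a movement showcase and launches the selected movement mode.
; On BeginPlay it disables the owning vehicle's input; starting a showcase sets the indexed movement pawn class on BP_GameMode and respawns the vehicle's controller.
; Getters expose the name, prompt, cameras, movement list and UI control definitions, plus the owner's BP_ShowcaseControlsInterface.
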(event `self.ReceiveBeginPlay`
  ;[1 1 1] Disables actor input on start
  (`/Game/VigilanteMovement/Shared/Blueprints/Base/BP_BaseVehicle.SetInputEnabled` (`self.GetBaseVehicle`) false))

(event `/Game/VigilanteMovement/Shared/Blueprints/HUD/Showcase/Interfaces/BP_ShowcaseSetupInterface.StartMovementShowcase`
  (params (Index :type Integer))
  (`self.Start Movement Mode` Index))

(fn `GetBaseVehicle`
  (returns (BaseVehicle :type "/Game/VigilanteMovement/Shared/Blueprints/Base/BP_BaseVehicle Object Reference"))
  (bind _asbp_base_vehicle (cast `/Game/VigilanteMovement/Shared/Blueprints/Base/BP_BaseVehicle` (`self.GetOwner`)))
  (return _asbp_base_vehicle))

(fn `GetButtonListControls`
  (returns (ButtonListControls :type "Array of /Game/VigilanteMovement/Shared/Blueprints/HUD/Showcase/Component/FButtonsControls Structure"))
  (return (`self.ButtonsControls`)))

(fn `GetCheckboxControls`
  (returns (CheckboxControls :type "Array of /Game/VigilanteMovement/Shared/Blueprints/HUD/Showcase/Component/FCheckboxControls Structure"))
  (return (`self.CheckboxControls`)))

(fn `GetMovementPromptText`
  (returns (Text :type Text))
  (return (`self.Prompt`)))

(fn `GetSeparators`
  (returns (Separators :type "Array of /Game/VigilanteMovement/Shared/Blueprints/HUD/Showcase/Component/FSeparator Structure"))
  (return (`self.Separators`)))

(fn `GetShowcaseCamera`
  (params (Index :type Integer))
  (returns (Camera :type "CameraActor Object Reference"))
  (return (`|GetArrayItem` (`self.ShowcaseCameras`) Index)))

(fn `GetShowcaseCameraCount`
  (returns (Count :type Integer))
  (return (`KismetArrayLibrary.Array_Length` (`self.ShowcaseCameras`))))

(fn `GetShowcaseControls`
  (returns (ControlsInterface :type "/Game/VigilanteMovement/Shared/Blueprints/HUD/Showcase/Interfaces/BP_ShowcaseControlsInterface Interface"))
  (bind _returnvalue (`self.GetOwner`))
  (if (`KismetSystemLibrary.DoesImplementInterface` _returnvalue "/Game/VigilanteMovement/Shared/Blueprints/HUD/Showcase/Interfaces/BP_ShowcaseControlsInterface.BP_ShowcaseControlsInterface_C")
    (bind _asbp_showcase_controls_interface (cast `/Game/VigilanteMovement/Shared/Blueprints/HUD/Showcase/Interfaces/BP_ShowcaseControlsInterface` (`self.GetOwner`)))
    (else
      (`KismetSystemLibrary.PrintString` (`KismetStringLibrary.Concat_StrStr` "Showcase Controls interface not supported in actor: " (`KismetStringLibrary.Conv_ObjectToString` _returnvalue)))))
  (return _asbp_showcase_controls_interface))

(fn `GetShowcaseMovements`
  (returns (MovementTypes :type "Array of /Game/VigilanteMovement/Shared/Blueprints/HUD/Showcase/Component/FShowcaseMovementSetup Structure"))
  (return (`self.MovementPawns`)))

(fn `GetShowcaseName`
  (returns (Name :type String))
  (return (`self.Name`)))

(fn `GetShowcaseSlot`
  (returns (Slot :type Integer))
  (return 0))

(fn `GetSliderControls`
  (returns (SliderControls :type "Array of /Game/VigilanteMovement/Shared/Blueprints/HUD/Showcase/Component/FSliderControls Structure"))
  (return (`self.SliderControls`)))

(fn `GetTwinSliderControls`
  (returns (TwinSliderControls :type "Array of /Game/VigilanteMovement/Shared/Blueprints/HUD/Showcase/Component/FTwinSliderControls Structure"))
  (return (`self.TwinSliderControls`)))

(fn `Start Movement Mode`
  (params (Index :type Integer))
  (bind _class (break `/Game/VigilanteMovement/Shared/Blueprints/HUD/Showcase/Component/FShowcaseMovementSetup` (`|GetArrayItem` (`self.MovementPawns`) Index)))
  (if (`KismetSystemLibrary.IsValidClass` _class)
    (bind _asbp_game_mode (cast `/Game/VigilanteMovement/Shared/Blueprints/GameMode/BP_GameMode` (`GameplayStatics.GetGameMode`)))
    (`/Game/VigilanteMovement/Shared/Blueprints/GameMode/BP_GameMode.SetMovementPawnClass` _asbp_game_mode _class)
    (`/Game/VigilanteMovement/Shared/Blueprints/GameMode/BP_GameMode.Respawn` _asbp_game_mode (`Pawn.GetController` (`self.GetBaseVehicle`)))
    (else
      (`KismetSystemLibrary.PrintString` "Unable to start movement mode due to invalid Movement Pawn Class" true true (struct :`R` 1.0 :`A` 1.0)))))