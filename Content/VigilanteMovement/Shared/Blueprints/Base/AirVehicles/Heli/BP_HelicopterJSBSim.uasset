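; Base helicopter Blueprint that layers flight inputs, gear, canopy, flashing lights and camera behavior onto a JSBSim-driven parent.
; Each tick writes Throttle to the JSBSim collective property, then calls collective and main-rotor hooks.
; Empty events let child Blueprints and their animation handle visuals and aiming, while FlipFlops drive timelines for gear, canopy and lights.
; Zoom inputs reposition the fixed cockpit camera, and secondary-camera switching can hide the HUD.
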(event `self.ReceiveTick`
  (params (DeltaSeconds :type "Float (single-precision)"))
  (`parent.ReceiveTick` DeltaSeconds)
  (`self.UpdateCollectiveJSBSim`)
  (`self.UpdateMainRotor` 0.0))

(event `SetCollective`
  ;[1 1 1] Used by Child Actor VFX and ABP
)

(event `self.ReceiveBeginPlay`
  (`parent.ReceiveBeginPlay`)
  ;[1 1 1] Set the lights to flash
  (`self.ToggleLights`)
  (`TimelineComponent.SetPlayRate` (`self.LightsFlash`) 0.3))

(event `UpdateMainRotor`
  (params (Value :type "Float (double-precision)"))
  ;[1 1 1] Used by Child Actor VFX and ABP
)

(event `SetGear`
  (params (Value :type "Float (double-precision)"))
  ;[1 1 1] Used by Child Actor VFX and ABP
)

(event `SetCanopy`
  (params (Value :type "Float (double-precision)"))
  ;[1 1 1] Used by Child Actor VFX and ABP
)

(event `UpdateYaw`
  (params (AxisValue :type "Float (double-precision)"))
  ;[1 1 1] Updates Yaw based on Input
  (bind _output_get (set `self.Yaw` AxisValue))
  (`self.SetYaw` _output_get))

(event `UpdateRoll`
  (params (AxisValue :type "Float (double-precision)"))
  ;[1 1 1] Updates Roll based on Input
  (bind _output_get (set `self.Roll` AxisValue))
  (`self.SetRoll` _output_get))

(event `UpdatePitch`
  (params (AxisValue :type "Float (double-precision)"))
  ;[1 1 1] Updates Pitch based on Input
  (bind _output_get (set `self.Pitch` AxisValue))
  (`self.SetPitch` _output_get))

(event `UpdateThrottle`
  (params (AxisValue :type "Float (double-precision)"))
  ;[1 1 1] Updates Throttle and Collective for Child ABP
  (set `self.Collective` AxisValue)
  (`self.SetCollective`))

(event `ToggleGear`
  ;[1 1 1] Toggles Gear (non JSBSim)
  (`/Engine/EditorBlueprintResources/StandardMacros.FlipFlop`
    (:`A`
      (bind (_direction _cu_simplecurve) (`Timeline|GearPosition` :!label _label)
        (:`Update`
          (`self.SetGear` _cu_simplecurve))))
    (:`B`
      (goto _label :!via `Reverse`))))

(event `ToggleLights`
  ;[1 1 1] Sets Lights on flashing or off
  (`/Engine/EditorBlueprintResources/StandardMacros.FlipFlop`
    (:`A`
      (bind (_direction _cu_sinus) (`Timeline|LightsFlash` :!via `PlayFromStart` :!label _label_2)
        (:`Update`
          (`self.SetLightsIntensity` _cu_sinus))))
    (:`B`
      (`self.SetLightsIntensity` 0.0)
      (goto _label_2 :!via `Stop`))))

(event `ToggleCanopy`
  ;[1 1 1] Toggles Canopy Open Close
  (`/Engine/EditorBlueprintResources/StandardMacros.FlipFlop`
    (:`A`
      (bind (_direction _cu_simplecurve) (`Timeline|CanopyPosition` :!label _label_3)
        (:`Update`
          (`self.SetCanopy` _cu_simplecurve))))
    (:`B`
      (goto _label_3 :!via `Reverse`))))

(event `InputAction|Zoom +`
  (params (Key :type "Key Structure"))
  ;[1 1 1] Switches between Seats or Zooms depending on specific vehicle child actor
  (:`Pressed`
    (if (`ActorComponent.IsActive` (`self.FixedCamera`))
      (`SceneComponent.K2_SetRelativeLocationAndRotation` (`self.FixedCamera`) (.location (`self.CockpitCameraZoomedTransform`)) (.rotation (`self.CockpitCameraZoomedTransform`)) false true)
      (set `CameraComponent.FieldOfView` (`self.CockpitCameraZoomedFOV`) (`self.FixedCamera`)))))

(event `InputAction|Zoom -`
  (params (Key :type "Key Structure"))
  ;[1 1 1] Switches between Seats or Zooms depending on specific vehicle child actor
  (:`Pressed`
    (if (`ActorComponent.IsActive` (`self.FixedCamera`))
      (`SceneComponent.K2_SetRelativeLocationAndRotation` (`self.FixedCamera`) (.location (`self.CockpitCameraUnZoomedTransform`)) (.rotation (`self.CockpitCameraUnZoomedTransform`)) false true)
      (set `CameraComponent.FieldOfView` (`self.CockpitCameraUnZoomedFOV`) (`self.FixedCamera`)))))

(event `UpdateAim`
  ;[1 1 1] Used by Child Actor BP to update specific Gun Rotation
)

(fn `SetActiveCamera`
  (params (bIsSecondaryCamera :type Boolean))
  ;[1 1 1] Switches between active cameras
  (`parent.SetActiveCamera` bIsSecondaryCamera)
  (if (`self.HideHUDOnSecondaryCam`)
    (`/Game/VigilanteMovement/Shared/Blueprints/HUD/Widget/BP_WidgetCommunicator.SetVehicleWIdgetVisibility` (`self.WidgetCommunicator`) (select `bool` bIsSecondaryCamera :`false` "Visible" :`true` "Hidden" :!type "ESlateVisibility Enum"))))

(fn `UpdateCollectiveJSBSim`
  ;[1 1 1] Updates Collecive Property in JSBsim based on Throttle input
  (`BlueprintMapLibrary.Map_Add` (`self.DoubleProperties`) (`self.CollectiveProperty`) (`self.Throttle`))
  (`self.UpdateThrottle` (`self.Throttle`)))

(fn `UserConstructionScript`
  (`parent.UserConstructionScript`))