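; Base helicopter vehicle that turns pilot input into flight, with empty events for child Blueprints to drive visuals and aiming.
; Axis inputs rotate the actor with pitch and roll bank limits, while throttle sets collective and starts a timeline-driven rotor spool-up.
; Thrust, tilt and gravity yield a velocity written to ProjectileMovement, with optional arcade lift.
; It also handles gear, canopy, flashing lights, cockpit zoom and rotor dust gated by a timed sphere trace.
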(event `self.ReceiveTick`
  (params (DeltaSeconds :type "Float (single-precision)"))
  (`parent.ReceiveTick` DeltaSeconds)
  (`self.UpdateDust`))

(event `self.ReceiveBeginPlay`
  ;[1 1 1] Sets Terrain Detection for Dust VFX
  (`KismetSystemLibrary.K2_SetTimer` null "Detect Terrain" 0.1 true)
  ;[1 1 1] Set the lights to flash
  (`self.ToggleLights`)
  (`TimelineComponent.SetPlayRate` (`self.LightsFlash`) 0.3))

(event `UpdateYaw`
  (params (AxisValue :type "Float (double-precision)"))
  ;[1 1 1] Updates Yaw based on Input
  (set `self.Yaw` AxisValue)
  (`self.SetYaw` (`self.Yaw`))
  (if (`self.isFlying`)
    (`self.K2_AddActorLocalRotation` (`KismetMathLibrary.MakeRotator` 0.0 0.0 (* (`self.Yaw`) (`self.YawMaxTurnRate`))))))

(event `SetYaw`
  (params (Value :type "Float (double-precision)"))
  ;[1 1 1] Used by Child Actor VFX and ABP
)

(event `UpdateRoll`
  (params (AxisValue :type "Float (double-precision)"))
  ;[1 1 1] Updates Roll based on Input
  (set `self.Roll` AxisValue)
  (`self.SetRoll` (`self.Roll`))
  (if (`self.isFlying`)
    ;[1 1 1] Checks if Helicopter does not exceeds Bank limits
    (if (or (and (> (`self.Roll`) 0.0) (>= (`self.BankLimit`) (.roll (`self.K2_GetActorRotation`)))) (and (< (`self.Roll`) 0.0) (<= (* (`self.BankLimit`) -1.0) (.roll (`self.K2_GetActorRotation`)))))
      ;[1 1 1] Rolls the helicopter
      (`self.K2_AddActorLocalRotation` (`KismetMathLibrary.MakeRotator` (* (`self.Roll`) (`self.RollMaxTurnRate`)))))))

(event `SetRoll`
  (params (Value :type "Float (double-precision)"))
  ;[1 1 1] Used by Child Actor VFX and ABP
)

(event `UpdatePitch`
  (params (AxisValue :type "Float (double-precision)"))
  ;[1 1 1] Updates Pitch based on Input
  (set `self.Pitch` AxisValue)
  (`self.SetPitch` (`self.Pitch`))
  (if (`self.isFlying`)
    ;[1 1 1] Checks is Helicopter does not exceeds Bank limits
    (if (or (and (> (`self.Pitch`) 0.0) (>= (`self.BankLimit`) (.pitch (`self.K2_GetActorRotation`)))) (and (< (`self.Pitch`) 0.0) (<= (* (`self.BankLimit`) -1.0) (.pitch (`self.K2_GetActorRotation`)))))
      ;[1 1 1] Sets the helicopter pitch
      (`self.K2_AddActorLocalRotation` (`KismetMathLibrary.MakeRotator` 0.0 (* (`self.Pitch`) (`self.PitchMaxTurnRate`)))))))

(event `SetPitch`
  (params (Pitch :type "Float (double-precision)"))
  ;[1 1 1] Used by Child Actor VFX and ABP
)

(event `UpdateThrottle`
  (params (AxisValue :type "Float (double-precision)"))
  ;[1 1 1] Updates Throttle
  (set `self.Collective` (`KismetMathLibrary.FClamp` (+ (* AxisValue (`self.CollectiveRate`)) (`self.Collective`))))
  ;[1 1 1] Starts the engine on throttle input if engine is off
  (if (not (`KismetMathLibrary.BooleanNOR` (`self.GetEngineState`) (!= (`self.Collective`) 0.0)))
    (`self.StartEngine`))
  (`self.UpdateSpeed`)
  (`self.SetCollective`))

(event `SetCollective`
  ;[1 1 1] Used by Child Actor VFX and ABP
)

(event `StartEngine`
  ;[1 1 1] Starts the Engine and set it to 100% RPM for rotors
  (`TimelineComponent.SetPlayRate` (`self.EngineRPS`) 0.1)
  (`self.SetEngineState` true)
  (bind (_direction _cu_smooth_simplecurve) (`Timeline|EngineRPS`)
    (:`Update`
      (bind _output_get (set `self.RotorMainRPS` _cu_smooth_simplecurve))
      (`self.UpdateMainRotor` _output_get))
    (:`Finished`
      (set `self.isFlying` true))))

(event `UpdateMainRotor`
  (params (Value :type "Float (double-precision)"))
  ;[1 1 1] Used by Child Actor VFX and ABP
)

(event `UpdateSpeed`
  ;[1 1 1] Does Flight Calculations
  (if (`self.isFlying`)
    (`self.Update Engine Trust`)
    (`self.Update Rotor Up`)
    (`self.Update Up Velocity`)
    (`self.Update Forward Velocity`)
    (`self.Update Side Velocity`)
    ;[1 1 1] Feeds Calculated Vectors to Projectile Movement
    (set `MovementComponent.Velocity` (`KismetMathLibrary.MakeVector` (.x (`KismetMathLibrary.TransformDirection` (`self.GetTransform`) (`KismetMathLibrary.MakeVector` (`self.ForwardSpeed`) (`self.RightSpeed`)))) (.y (`KismetMathLibrary.TransformDirection` (`self.GetTransform`) (`KismetMathLibrary.MakeVector` (`self.ForwardSpeed`) (`self.RightSpeed`)))) (`self.WorldUpSpeed`)) (`self.ProjectileMovement`))))

(event `ToggleGear`
  ;[1 1 1] Toggles Gear
  (`/Engine/EditorBlueprintResources/StandardMacros.FlipFlop`
    (:`A`
      (bind (_direction _cu_simplecurve) (`Timeline|GearPosition` :!label _label)
        (:`Update`
          (bind _output_get (set `self.GearsValue` _cu_simplecurve))
          (`self.SetGear` _output_get))))
    (:`B`
      (goto _label :!via `Reverse`))))

(event `SetGear`
  (params (Value :type "Float (double-precision)"))
  ;[1 1 1] Used by Child Actor VFX and ABP
)

(event `ToggleLights`
  ;[1 1 1] Sets Lights on flashing or off
  (`/Engine/EditorBlueprintResources/StandardMacros.FlipFlop`
    (:`A`
      (bind (_direction _cu_sinus) (`Timeline|LightsFlash` :!via `PlayFromStart` :!label _label_2)
        (:`Update`
          (`self.SetLightsIntensity` _cu_sinus))))
    (:`B`
      (`self.SetLightsIntensity` 0.0)
      (goto _label_2 :!via `Stop`))))

(event `ToggleCanopy`
  ;[1 1 1] Toggles Canopy Open Close
  (`/Engine/EditorBlueprintResources/StandardMacros.FlipFlop`
    (:`A`
      (bind (_direction _cu_simplecurve) (`Timeline|CanopyPosition` :!label _label_3)
        (:`Update`
          (`self.SetCanopy` _cu_simplecurve))))
    (:`B`
      (goto _label_3 :!via `Reverse`))))

(event `SetCanopy`
  (params (Value :type "Float (double-precision)"))
  ;[1 1 1] Used by Child Actor VFX and ABP
)

(event `InputAction|Zoom +`
  (params (Key :type "Key Structure"))
  ;[1 1 1] Switches between Seats or Zooms depending on specific vehicle child actor
  (:`Pressed`
    (if (`ActorComponent.IsActive` (`self.FixedCamera`))
      (`SceneComponent.K2_SetRelativeLocationAndRotation` (`self.FixedCamera`) (.location (`self.CockpitCameraZoomedTransform`)) (.rotation (`self.CockpitCameraZoomedTransform`)) false true)
      (set `CameraComponent.FieldOfView` (`self.CockpitCameraZoomedFOV`) (`self.FixedCamera`)))))

(event `InputAction|Zoom -`
  (params (Key :type "Key Structure"))
  ;[1 1 1] Switches between Seats or Zooms depending on specific vehicle child actor
  (:`Pressed`
    (if (`ActorComponent.IsActive` (`self.FixedCamera`))
      (`SceneComponent.K2_SetRelativeLocationAndRotation` (`self.FixedCamera`) (.location (`self.CockpitCameraUnZoomedTransform`)) (.rotation (`self.CockpitCameraUnZoomedTransform`)) false true)
      (set `CameraComponent.FieldOfView` (`self.CockpitCameraUnZoomedFOV`) (`self.FixedCamera`)))))

(event `UpdateAim`
  ;[1 1 1] Used by Child Actor BP to update specific Gun Rotation
)

(event `InputAxis|Thrust`
  (params (AxisValue :type "Float (single-precision)"))
  (`self.UpdateThrottle` AxisValue))

(event `InputAxis|MoveRight`
  (params (AxisValue :type "Float (single-precision)"))
  (`self.UpdateYaw` AxisValue))

(event `InputAxis|Roll`
  (params (AxisValue :type "Float (single-precision)"))
  (`self.UpdateRoll` AxisValue))

(event `InputAxis|Pitch`
  (params (AxisValue :type "Float (single-precision)"))
  (if (`self.InvertPitch`)
    (`self.UpdatePitch` (* AxisValue -1.0))
    (else
      (`self.UpdatePitch` AxisValue))))

(event `InputAction|Gears`
  (params (Key :type "Key Structure"))
  (:`Pressed`
    (`self.ToggleGear`)))

(event `InputAction|Open Canopy`
  (params (Key :type "Key Structure"))
  (:`Pressed`
    (`self.ToggleCanopy`)))

(event `InputAxis|LookUp`
  (params (AxisValue :type "Float (single-precision)"))
  (`self.UpdateAim`))

(event `InputAxis|LookAround`
  (params (AxisValue :type "Float (single-precision)"))
  (`self.UpdateAim`))

(fn `Detect Terrain`
  (bind _returnvalue (`self.K2_GetActorLocation`))
  ;[1 1 1] Detects Terrain and Obstacles to spawn Dust Whirl VFX
  (bind (_outhits _returnvalue_2) (`KismetSystemLibrary.SphereTraceMulti` _returnvalue (+ _returnvalue (`self.TerrainDetectionOffset`)) (`self.TerrainDetectionRadius`) "TraceTypeQuery1"))
  (if _returnvalue_2
    (set `self.ShowDust` true)
    (else
      (set `self.ShowDust` false))))

(fn `SetActiveCamera`
  (params (bIsSecondaryCamera :type Boolean))
  ;[1 1 1] Switches between active cameras
  (`parent.SetActiveCamera` bIsSecondaryCamera)
  (if (`self.HideHUDOnSecondaryCam`)
    (`/Game/VigilanteMovement/Shared/Blueprints/HUD/Widget/BP_WidgetCommunicator.SetVehicleWIdgetVisibility` (`self.WidgetCommunicator`) (select `bool` bIsSecondaryCamera :`false` "Visible" :`true` "Hidden" :!type "ESlateVisibility Enum"))))

(fn `Update Engine Trust`
  ;[1 1 1] Updates Engine Thrust based on RPS and Throttle
  (set `self.EngineThurst` (* (`self.Collective`) (`self.RotorMainRPS`))))

(fn `Update Forward Velocity`
  (set `self.ForwardSpeed` (* (* (`self.RotorUpSpeed`) (* (`KismetMathLibrary.DegCos` (.roll (`self.K2_GetActorRotation`))) (* (`KismetMathLibrary.DegSin` (.pitch (`self.K2_GetActorRotation`))) -1.0))) (`self.ForwardSpeedMultiplicator`))))

(fn `Update Rotor Up`
  ;[1 1 1] Updates Rotor Up Thrust
  (set `self.RotorUpSpeed` (* (`self.EngineThurst`) (`self.UpRate`) (* (`self.Gravity`) -2.0))))

(fn `Update Side Velocity`
  (set `self.RightSpeed` (* (* (`self.RotorUpSpeed`) (* (`KismetMathLibrary.DegSin` (.roll (`self.K2_GetActorRotation`))) (`KismetMathLibrary.DegCos` (.pitch (`self.K2_GetActorRotation`))))) (`self.RightSpeedMultiplicator`))))

(fn `Update Up Velocity`
  ;[1 1 1] Arcade mode Inclination does not affect Up Velocity
  (if (not (`self.ArcadeInclination`))
    (set `self.ImpactInclinationOnUp` (* (`KismetMathLibrary.DegCos` (.roll (`self.K2_GetActorRotation`))) (`KismetMathLibrary.DegCos` (.pitch (`self.K2_GetActorRotation`))))))
  ;[1 1 1] Calculates Up Velocity
  (set `self.WorldUpSpeed` (* (`self.RotorUpSpeed`) (`self.ImpactInclinationOnUp`)))
  ;[1 1 1] Effect of Gravity
  (set `self.WorldUpSpeed` (+ (`self.WorldUpSpeed`) (`self.Gravity`))))

(fn `UpdateDust`
  (if (`self.ShowDust`)
    (`NiagaraComponent.SetVariableFloat` (`self.DownwardDust`) "PropSpeed" (* (`self.RotorMainRPS`) (`self.DustMultiplicator`)))
    (else
      (`NiagaraComponent.SetVariableFloat` (`self.DownwardDust`) "PropSpeed" 0.0))))

(fn `UserConstructionScript`
  (`parent.UserConstructionScript`))