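; Base airplane Blueprint driven by JSBSim flight dynamics, with hooks for child Blueprints and animation.
; Each tick it writes throttle and afterburner augmentation into every JSBSim engine command, caches per-engine afterburner state, then fires throttle and afterburner events.
; Input sets pitch, roll and yaw, toggles timeline-driven flashing lights and canopy, and switches cockpit camera zoom.
; Switching to the secondary camera can hide the vehicle HUD.
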(event `self.ReceiveTick`
  (params (DeltaSeconds :type "Float (single-precision)"))
  ;[1 1 1] Initial States
  (`parent.ReceiveTick` DeltaSeconds)
  (`self.UpdateJSBSimEngines`)
  (`self.SetAfterburner`))

(event `self.ReceiveBeginPlay`
  (`parent.ReceiveBeginPlay`))

(event `SetThrottle`
  ;[1 1 1] Used by Child Actor VFX and ABP
)

(event `SetAfterburner`
  ;[1 1 1] Used by Child Actor VFX and ABP
)

(event `UpdateYaw`
  (params (AxisValue :type "Float (double-precision)"))
  ;[1 1 1] Updates Yaw based on Input
  (bind _output_get (set `self.Yaw` AxisValue))
  (`self.SetYaw` _output_get))

(event `SetCanopy`
  (params (Value :type "Float (double-precision)"))
  ;[1 1 1] Used by Child Actor VFX and ABP
)

(event `UpdateRoll`
  (params (AxisValue :type "Float (double-precision)"))
  ;[1 1 1] Updates Roll based on Input
  (bind _output_get (set `self.Roll` AxisValue))
  (`self.SetRoll` _output_get))

(event `UpdatePitch`
  (params (AxisValue :type "Float (double-precision)"))
  ;[1 1 1] Updates Pitch based on Input
  (bind _output_get (set `self.Pitch` AxisValue))
  (`self.SetPitch` _output_get))

(event `ToggleLights`
  ;[1 1 1] Sets Lights on flashing or off
  (`/Engine/EditorBlueprintResources/StandardMacros.FlipFlop`
    (:`A`
      (bind (_direction _cu_sinus) (`Timeline|LightsFlash` :!via `PlayFromStart` :!label _label)
        (:`Update`
          (`self.SetLightsIntensity` _cu_sinus))))
    (:`B`
      (`self.SetLightsIntensity` 0.0)
      (goto _label :!via `Stop`))))

(event `ToggleCanopy`
  ;[1 1 1] Toggles Canopy Open Close
  (`/Engine/EditorBlueprintResources/StandardMacros.FlipFlop`
    (:`A`
      (bind (_direction _cu_simplecurve) (`Timeline|CanopyPosition` :!label _label_2)
        (:`Update`
          (`self.SetCanopy` _cu_simplecurve))))
    (:`B`
      (goto _label_2 :!via `Reverse`))))

(event `InputAction|Zoom +`
  (params (Key :type "Key Structure"))
  ;[1 1 1] Switches between Seats or Zooms depending on specific vehicle child actor
  (:`Pressed`
    (if (`ActorComponent.IsActive` (`self.FixedCamera`))
      (`SceneComponent.K2_SetRelativeLocationAndRotation` (`self.FixedCamera`) (.location (`self.CockpitCameraZoomedTransform`)) (.rotation (`self.CockpitCameraZoomedTransform`)) false true)
      (set `CameraComponent.FieldOfView` (`self.CockpitCameraZoomedFOV`) (`self.FixedCamera`)))))

(event `InputAction|Zoom -`
  (params (Key :type "Key Structure"))
  ;[1 1 1] Switches between Seats or Zooms depending on specific vehicle child actor
  (:`Pressed`
    (if (`ActorComponent.IsActive` (`self.FixedCamera`))
      (`SceneComponent.K2_SetRelativeLocationAndRotation` (`self.FixedCamera`) (.location (`self.CockpitCameraUnZoomedTransform`)) (.rotation (`self.CockpitCameraUnZoomedTransform`)) false true)
      (set `CameraComponent.FieldOfView` (`self.CockpitCameraUnZoomedFOV`) (`self.FixedCamera`)))))

(event `UpdateAim`
  ;[1 1 1] Used by Child Actor BP to update specific Gun Rotation
)

(event `InputAction|Boost`
  (params (Key :type "Key Structure"))
  ;[1 1 1] Afterburner for Engines Agumentation Method 0
  (:`Pressed`
    (set `self.Augmentation` true))
  (:`Released`
    (set `self.Augmentation` false)))

(fn `SetActiveCamera`
  (params (bIsSecondaryCamera :type Boolean))
  ;[1 1 1] Switches between active cameras
  (`parent.SetActiveCamera` bIsSecondaryCamera)
  (if (`self.HideHUDOnSecondaryCam`)
    (`/Game/VigilanteMovement/Shared/Blueprints/HUD/Widget/BP_WidgetCommunicator.SetVehicleWIdgetVisibility` (`self.WidgetCommunicator`) (select `bool` bIsSecondaryCamera :`false` "Visible" :`true` "Hidden" :!type "ESlateVisibility Enum"))))

(fn `UpdateJSBSimEngines`
  (locals (L_Index :type Integer))
  (`KismetArrayLibrary.Array_Clear` (`self.isAfterburnerActive`))
  (for (_array_element _array_index) (`/Game/VigilanteMovement/Shared/Blueprints/Base/AirVehicles/Airplane/BP_Airplane_JSBSim.EngineCommands` (`self.JSBSimMovement`))
    (set `local.L_Index` _array_index)
    (bind (_mixture _starter _running _propelleradvance _propellerfeather _magnetos _injection _ignition _reverse _cutoff _generatorpower _condition) (break `` _array_element))
    ;[1 1 1] Updates JSBSim Engines Commands
    (`KismetArrayLibrary.Array_Set` (`/Game/VigilanteMovement/Shared/Blueprints/Base/AirVehicles/Airplane/BP_Airplane_JSBSim.EngineCommands` (`self.JSBSimMovement`)) (`local.L_Index`) (make `` (`self.Throttle`) _mixture _starter _running _propelleradvance _propellerfeather _magnetos (`self.Augmentation`) _injection _ignition _reverse _cutoff _generatorpower _condition))
    ;[1 1 1] Updates Engine States - Afterburner
    (`KismetArrayLibrary.Array_Add` (`self.isAfterburnerActive`) (`.Augmentation` (break `` (`|GetArrayItem` (`/Game/VigilanteMovement/Shared/Blueprints/Base/AirVehicles/Airplane/BP_Airplane_JSBSim.EngineStates` (`self.JSBSimMovement`)) (`local.L_Index`))))))
  ;[1 1 1] Calls Event for Child BP and ABP
  (`self.SetThrottle`))

(fn `UserConstructionScript`
  (`parent.UserConstructionScript`))