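; Base airplane vehicle providing arcade flight with optional VTOL and afterburner, plus cockpit camera zoom.
; Throttle input runs thrust, speed, drag and curve-based lift calculations that set ProjectileMovement velocity, while steering applies local rotations.
; FlipFlop-driven timelines animate gear, flaps, air brake and other parts, passing values through empty Set events, some noted for child VFX and animation.
; A looping sphere trace enables throttle-scaled dust, and fired projectiles inherit the plane's velocity.
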(event `self.ReceiveBeginPlay`
  (`|ExecutionSequence`
    (:`then_0`
      ;[1 1 1] Sets Top Speed as Marginal Velocity
      (set `self.MarginalVelocity` (`self.TopSpeed`)))
    (:`then_1`
      ;[1 1 1] Switchs on Lights and blinks
      (`self.ToggleLights`)
      (`TimelineComponent.SetPlayRate` (`self.LightsBlink`) 0.3))
    (:`then_2`
      ;[1 1 1] Sets proper initial values for flight
      (`KismetSystemLibrary.Delay` 0.1)
      (if (`self.isFlying`)
        (set `self.Throttle` 0.3)
        (set `self.ForwardSpeed` 9000.0)
        (`self.ToggleGear`)
        (`ActorComponent.SetActive` (`self.ProjectileMovement`) true true)))
    (:`then_3`
      ;[1 1 1] Sets Terrain Detection for Dust VFX
      (`KismetSystemLibrary.K2_SetTimer` null "DetectTerrain" 0.1 true))))

(event `self.ReceiveTick`
  (params (DeltaSeconds :type "Float (single-precision)"))
  (`parent.ReceiveTick` DeltaSeconds)
  (`self.UpdateDust`))

(event `UpdateThrottle`
  (params (AxisValue :type "Float (double-precision)"))
  ;[1 1 1] Updates Throttle
  (set `self.Throttle` (`KismetMathLibrary.FClamp` (+ (* AxisValue (`self.ThrottleRate`)) (`self.Throttle`))))
  (`self.UpdateSpeed`)
  (`self.SetThrottle`))

(event `SetThrottle`
  ;[1 1 1] Used by Child Actor VFX and ABP
)

(event `UpdateSpeed`
  ;[1 1 1] Does Flight Calculations
  (`self.Update Engine Trust`)
  (`self.Update Forward Velocity`)
  (`self.Update VTOLImpact`)
  (`self.Update Drag`)
  ;[1 1 1] Feeds Calculated Vectors to Projectile Movement
  (`ProjectileMovementComponent.SetVelocityInLocalSpace` (`self.ProjectileMovement`) (+ (`KismetMathLibrary.MakeVector` (`KismetMathLibrary.FClamp` (`self.ForwardSpeed`) 0.0 (`self.MarginalVelocity`)) (`self.RightSpeed`) (`self.UpSpeed`)) (`KismetMathLibrary.InverseTransformDirection` (`self.GetTransform`) (`self.Update Lift`)))))

(event `ToggleAfterburner`
  (params (SetActive :type Boolean))
  ;[1 1 1] Handels Afterburner
  (if (`self.hasAfterburner`)
    (if SetActive
      (if (== (`self.VTOLRatio`) 0.0)
        (set `self.isAfterburnerActive` true)
        (set `self.MarginalVelocity` (`self.TopSpeedAF`))
        (`self.SetAfterburner` :!label _label))
      (else
        (set `self.isAfterburnerActive` false)
        (set `self.MarginalVelocity` (`self.TopSpeed`))
        (goto _label)))))

(event `SetAfterburner`
  ;[1 1 1] Used by Child Actor VFX and ABP
)

(event `UpdateYaw`
  (params (AxisValue :type "Float (double-precision)"))
  ;[1 1 1] Updates Airplane Yaw Rotation
  (set `self.Yaw` AxisValue)
  (`self.K2_AddActorLocalRotation` (`KismetMathLibrary.MakeRotator` 0.0 0.0 (* (`self.Yaw`) (`self.YawMaxTurnRate`) (+ (/ (`self.ForwardSpeed`) (`self.MarginalVelocity`)) (`self.VTOLRatio`)))))
  (`self.SetYaw` (`self.Yaw`)))

(event `SetYaw`
  (params (Value :type "Float (double-precision)"))
  ;[1 1 1] Used by Child Actor VFX and ABP
)

(event `SetRoll`
  (params (Value :type "Float (double-precision)"))
  ;[1 1 1] Used by Child Actor VFX and ABP
)

(event `UpdateRoll`
  (params (AxisValue :type "Float (double-precision)"))
  ;[1 1 1] Updates Airplane Roll Rotation
  (set `self.Roll` AxisValue)
  (`self.K2_AddActorLocalRotation` (`KismetMathLibrary.MakeRotator` (* (`self.Roll`) (`self.RollMaxTurnRate`) (+ (/ (`self.ForwardSpeed`) (`self.MarginalVelocity`)) (`self.VTOLRatio`)))))
  (`self.SetRoll` (`self.Roll`)))

(event `UpdatePitch`
  (params (AxisValue :type "Float (double-precision)"))
  ;[1 1 1] Updates Airplane Pitch Rotation
  (set `self.Pitch` AxisValue)
  (`self.K2_AddActorLocalRotation` (`KismetMathLibrary.MakeRotator` 0.0 (* (`self.Pitch`) (+ (+ (* (`CurveFloat.GetFloatValue` (`self.PitchTurnRateCurve`) (`self.ForwardSpeed`)) (`GameplayStatics.GetWorldDeltaSeconds`)) 0.0) (`self.VTOLRatio`)))))
  (`self.SetPitch` (`self.Pitch`)))

(event `SetPitch`
  (params (Pitch :type "Float (double-precision)"))
  ;[1 1 1] Used by Child Actor VFX and ABP
)

(event `UpdateVTOLRatio`
  (params (Value :type "Float (double-precision)"))
  ;[1 1 1] Updates VTOL Vectoring Ratio
  (if (`self.isVTOL`)
    (bind _output_get (set `self.VTOLRatio` (`KismetMathLibrary.FClamp` (+ (`self.VTOLRatio`) (* Value 0.01)))))
    (`self.SetVTOLRatio` _output_get)
    (if (and (!= _output_get 0.0) (`self.isAfterburnerActive`))
      (`self.ToggleAfterburner` false))))

(event `SetVTOLRatio`
  (params (Value :type "Float (double-precision)"))
  ;[1 1 1] Used by Child Actor VFX and ABP
)

(event `ToggleGear`
  ;[1 1 1] Toggles Gear
  (`/Engine/EditorBlueprintResources/StandardMacros.FlipFlop`
    (:`A`
      (bind (_direction _cu_simplecurve) (`Timeline|GearPosition` :!label _label_2)
        (:`Update`
          (bind _output_get (set `self.GearsValue` _cu_simplecurve))
          (`self.SetGear` _output_get))))
    (:`B`
      (goto _label_2 :!via `Reverse`))))

(event `SetGear`
  (params (Value :type "Float (double-precision)"))
  ;[1 1 1] Used by Child Actor VFX and ABP
)

(event `ToggleFlaps`
  ;[1 1 1] Toggles Flaps
  (`/Engine/EditorBlueprintResources/StandardMacros.FlipFlop`
    (:`A`
      (bind (_direction _cu_simplecurve) (`Timeline|FlapsPosition` :!label _label_3)
        (:`Update`
          (bind _output_get (set `self.FlapsValue` _cu_simplecurve))
          (`self.SetFlaps` _output_get))))
    (:`B`
      (goto _label_3 :!via `Reverse`))))

(event `SetFlaps`
  (params (Value :type "Float (double-precision)"))
  ;[1 1 1] Used by Child Actor VFX and ABP
)

(event `ToggleAirBrake`
  ;[1 1 1] Toggles Air Brake
  (`/Engine/EditorBlueprintResources/StandardMacros.FlipFlop`
    (:`A`
      (bind (_direction _cu_simplecurve) (`Timeline|AirBrakePosition` :!label _label_4)
        (:`Update`
          (bind _output_get (set `self.AirBrakeValue` _cu_simplecurve))
          (`self.SetAirBrake` _output_get))))
    (:`B`
      (goto _label_4 :!via `Reverse`))))

(event `SetAirBrake`
  (params (Value :type "Float (double-precision)"))
  ;[1 1 1] Used by Child Actor VFX and ABP
)

(event `ToggleLights`
  ;[1 1 1] Toggles Lights
  (`/Engine/EditorBlueprintResources/StandardMacros.FlipFlop`
    (:`A`
      (bind (_direction _cu_sinus) (`Timeline|LightsBlink` :!via `PlayFromStart` :!label _label_5)
        (:`Update`
          (`self.SetLightsIntensity` _cu_sinus))))
    (:`B`
      (`self.SetLightsIntensity` 0.0 :!label _label_6)
      (goto _label_5 :!via `Stop`))))

(event `TurnOffLights`
  ;[1 1 1] Toggles Lights
  (goto _label_6))

(event `ToggleCanopy`
  ;[1 1 1] Toggles Canopy
  (`/Engine/EditorBlueprintResources/StandardMacros.FlipFlop`
    (:`A`
      (bind (_direction _cu_simplecurve) (`Timeline|CanopyPosition` :!label _label_7)
        (:`Update`
          (`self.SetCanopy` _cu_simplecurve))))
    (:`B`
      (goto _label_7 :!via `Reverse`))))

(event `SetCanopy`
  (params (Value :type "Float (double-precision)"))
  ;[1 1 1] Used by Child Actor VFX and ABP
)

(event `ToggleHook`
  ;[1 1 1] Toggles Landing Hook
  (`/Engine/EditorBlueprintResources/StandardMacros.FlipFlop`
    (:`A`
      (bind (_direction _cu_simplecurve) (`Timeline|HookPosition` :!label _label_8)
        (:`Update`
          (`self.SetHook` _cu_simplecurve))))
    (:`B`
      (goto _label_8 :!via `Reverse`))))

(event `SetHook`
  (params (Value :type "Float (double-precision)"))
  ;[1 1 1] Used by Child Actor VFX and ABP
)

(event `ToggleWings`
  ;[1 1 1] Toggles Foldable Wings
  (`/Engine/EditorBlueprintResources/StandardMacros.FlipFlop`
    (:`A`
      (bind (_direction _cu_simplecurve) (`Timeline|WingsPosition` :!label _label_9)
        (:`Update`
          (`self.SetWings` _cu_simplecurve))))
    (:`B`
      (goto _label_9 :!via `Reverse`))))

(event `SetWings`
  (params (Value :type "Float (double-precision)"))
  ;[1 1 1] Used by Child Actor VFX and ABP
)

(event `ToggleRefuel`
  ;[1 1 1] Toggles Refuel
  (`/Engine/EditorBlueprintResources/StandardMacros.FlipFlop`
    (:`A`
      (bind (_direction _cu_smooth_simplecurve) (`Timeline|RefuelPosition` :!label _label_10)
        (:`Update`
          (`self.SetRefuel` _cu_smooth_simplecurve))))
    (:`B`
      (goto _label_10 :!via `Reverse`))))

(event `SetRefuel`
  (params (Value :type "Float (double-precision)"))
  ;[1 1 1] Used by Child Actor VFX and ABP
)

(event `ToggleBombBay`
  ;[1 1 1] Toggles BombBay
  (`/Engine/EditorBlueprintResources/StandardMacros.FlipFlop`
    (:`A`
      (bind (_direction _cu_smooth_simplecurve) (`Timeline|BombBayPosition` :!label _label_11)
        (:`Update`
          (`self.SetBombBay` _cu_smooth_simplecurve))))
    (:`B`
      (goto _label_11 :!via `Reverse`))))

(event `SetBombBay`
  (params (Value :type "Float (double-precision)"))
  ;[1 1 1] Used by Child Actor VFX and ABP
)

(event `InputAction|Zoom +`
  (params (Key :type "Key Structure"))
  ;[1 1 1] Zooms Pilot Camera / Switchs Seats
  (:`Pressed`
    (if (`ActorComponent.IsActive` (`self.FixedCamera`))
      (`SceneComponent.K2_SetRelativeLocationAndRotation` (`self.FixedCamera`) (.location (`self.CockpitCameraZoomedTransform`)) (.rotation (`self.CockpitCameraZoomedTransform`)) false true)
      (set `CameraComponent.FieldOfView` (`self.CockpitCameraZoomedFOV`) (`self.FixedCamera`))
      (set `self.isCameraZoomed` true))))

(event `InputAction|Zoom -`
  (params (Key :type "Key Structure"))
  ;[1 1 1] Zooms Pilot Camera / Switchs Seats
  (:`Pressed`
    (if (`ActorComponent.IsActive` (`self.FixedCamera`))
      (`SceneComponent.K2_SetRelativeLocationAndRotation` (`self.FixedCamera`) (.location (`self.CockpitCameraUnZoomedTransform`)) (.rotation (`self.CockpitCameraUnZoomedTransform`)) false true)
      (set `CameraComponent.FieldOfView` (`self.CockpitCameraUnZoomedFOV`) (`self.FixedCamera`))
      (set `self.isCameraZoomed` false))))

(event `InputAxis|Thrust`
  (params (AxisValue :type "Float (single-precision)"))
  ;[1 1 1] Mapps Project Inputs to coresponding Events
  (`self.UpdateThrottle` AxisValue))

(event `InputAxis|MoveRight`
  (params (AxisValue :type "Float (single-precision)"))
  ;[1 1 1] Mapps Project Inputs to coresponding Events
  (`self.UpdateYaw` AxisValue))

(event `InputAxis|Roll`
  (params (AxisValue :type "Float (single-precision)"))
  ;[1 1 1] Mapps Project Inputs to coresponding Events
  (`self.UpdateRoll` AxisValue))

(event `InputAxis|Pitch`
  (params (AxisValue :type "Float (single-precision)"))
  ;[1 1 1] Mapps Project Inputs to coresponding Events
  (if (`self.InvertPitch`)
    (`self.UpdatePitch` (* AxisValue -1.0))
    (else
      (`self.UpdatePitch` AxisValue))))

(event `InputAxis|Lift`
  (params (AxisValue :type "Float (single-precision)"))
  ;[1 1 1] Mapps Project Inputs to coresponding Events
  (`self.UpdateVTOLRatio` AxisValue))

(event `InputAction|Flaps`
  (params (Key :type "Key Structure"))
  ;[1 1 1] Mapps Project Inputs to coresponding Events
  (:`Pressed`
    (`self.ToggleFlaps`)))

(event `InputAction|Gears`
  (params (Key :type "Key Structure"))
  ;[1 1 1] Mapps Project Inputs to coresponding Events
  (:`Pressed`
    (`self.ToggleGear`)))

(event `InputAction|Handbrake`
  (params (Key :type "Key Structure"))
  ;[1 1 1] Mapps Project Inputs to coresponding Events
  (:`Pressed`
    (`self.ToggleAirBrake`)))

(event `InputAction|Boost`
  (params (Key :type "Key Structure"))
  ;[1 1 1] Mapps Project Inputs to coresponding Events
  (:`Pressed`
    (`self.ToggleAfterburner` true))
  (:`Released`
    (`self.ToggleAfterburner` false)))

(event `InputAction|Hook`
  (params (Key :type "Key Structure"))
  ;[1 1 1] Mapps Project Inputs to coresponding Events
  (:`Pressed`
    (`self.ToggleHook`)))

(event `InputAction|Fold Wings`
  (params (Key :type "Key Structure"))
  ;[1 1 1] Mapps Project Inputs to coresponding Events
  (:`Pressed`
    (`self.ToggleWings`)))

(event `InputAction|Open Canopy`
  (params (Key :type "Key Structure"))
  ;[1 1 1] Mapps Project Inputs to coresponding Events
  (:`Pressed`
    (`self.ToggleCanopy`)))

(event `InputAction|Refuel`
  (params (Key :type "Key Structure"))
  ;[1 1 1] Mapps Project Inputs to coresponding Events
  (:`Pressed`
    (`self.ToggleRefuel`)))

(event `InputAction|OpenBay`
  (params (Key :type "Key Structure"))
  ;[1 1 1] Mapps Project Inputs to coresponding Events
  (:`Pressed`
    (`self.ToggleBombbay`)))

(fn `DetectTerrain`
  (bind _returnvalue (`self.K2_GetActorLocation`))
  ;[1 1 1] Detects Terrain and Obstacles to spawn Dust Whirl VFX
  (bind (_outhits _returnvalue_2) (`KismetSystemLibrary.SphereTraceMulti` _returnvalue (+ _returnvalue (`self.TerrainDetectionOffset`)) (`self.TerrainDetectionRadius`) "TraceTypeQuery1"))
  (if _returnvalue_2
    (set `self.ShowDust` true)
    (else
      (set `self.ShowDust` false))))

(fn `InitProjectile`
  (params (BaseProjectileMovement :type "ProjectileMovementComponent Object Reference"))
  (`parent.InitProjectile` BaseProjectileMovement)
  (set `MovementComponent.Velocity` (`MovementComponent.Velocity` (`self.ProjectileMovement`)) BaseProjectileMovement))

(fn `SetActiveCamera`
  (params (bIsSecondaryCamera :type Boolean))
  ;[1 1 1] Switches between External Vehicle View and Pilot Seat Cameras
  (`parent.SetActiveCamera` bIsSecondaryCamera)
  (if (`self.HideHMDOnSecondaryCam`)
    (`/Game/VigilanteMovement/Shared/Blueprints/HUD/Widget/BP_WidgetCommunicator.SetVehicleWIdgetVisibility` (`self.WidgetCommunicator`) (select `bool` bIsSecondaryCamera :`false` "Visible" :`true` "Hidden" :!type "ESlateVisibility Enum"))))

(fn `Update Drag`
  ;[1 1 1] Updates Drag based on Gears and AirBrake
  (set `self.ForwardSpeed` (* (- 1.0 (+ (* (- 1.0 (`self.GearsValue`)) (`self.GearsDragIndex`)) (* (`self.AirBrakeValue`) (`self.AirBrakeDragIndex`)))) (`self.ForwardSpeed`))))

(fn `Update Engine Trust`
  ;[1 1 1] Updates Thrust based on Throttle
  (set `self.EngineThrust` (`self.Throttle`)))

(fn `Update Forward Velocity`
  ;[1 1 1] Calculates Forward Velocity
  (set `self.ForwardSpeed` (+ (`self.ForwardSpeed`) (* (`self.AccelerationRate`) (* (/ (- (`self.ForwardSpeed`) (* (`self.MarginalVelocity`) (* (`self.EngineThrust`) (- 1.0 (`self.VTOLRatio`))))) (`self.MarginalVelocity`)) -1.0)))))

(fn `Update Lift`
  (returns (ReturnValue :type "Vector Structure"))
  ;[1 1 1] Updates Lift
  (return (`KismetMathLibrary.MakeVector` 0.0 0.0 (* (- 1.0 (`CurveFloat.GetFloatValue` (`self.LiftCurve`) (+ (`self.ForwardSpeed`) (* (* (`self.FlapsLiftIndex`) (`self.MarginalVelocity`)) (`self.FlapsValue`) (- 1.0 (`self.VTOLRatio`)))))) (`self.Gravity`)))))

(fn `Update VTOLImpact`
  ;[1 1 1] Calculates Impact of VTOL vector on Up Velocity
  (set `self.UpSpeed` (* (`self.MaxVTOLZSpeed`) (* (`self.EngineThrust`) (`self.VTOLRatio`)))))

(fn `UpdateDust`
  (if (`self.ShowDust`)
    (`NiagaraComponent.SetVariableFloat` (`self.DownwardDust`) "AirSpeed" (* (`self.Throttle`) (`self.DustMultiplicator`)))
    (else
      (`NiagaraComponent.SetVariableFloat` (`self.DownwardDust`) "AirSpeed" 0.0))))

(fn `UserConstructionScript`
  (`parent.UserConstructionScript`))