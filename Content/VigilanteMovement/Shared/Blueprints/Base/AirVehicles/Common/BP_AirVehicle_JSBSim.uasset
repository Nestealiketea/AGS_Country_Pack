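; Base Blueprint for JSBSim-driven air vehicles, with flight input, trim, gear, flap and brake controls.
; Input fills control variables and child hooks, but ApplyFlightCommands is empty here, its command write left unwired.
; Tick pushes property maps into JSBSim and reads back gear, wheel and RPM animation data, airspeed, altitude and crashes, which trigger damaged mode.
; A timed sphere trace flags dust VFX, and projectile initial speed scales with airspeed.
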(event `SetPitch`
  (params (PitchValue :type "Float (double-precision)"))
  ;[1 1 1] Events used by Child BP
)

(event `self.ReceiveBeginPlay`
  (bind _jsbsimmovement (`self.JSBSimMovement`))
  (`parent.ReceiveBeginPlay`)
  ;[1 1 1] Apply JSBSim Properties on Begin
  (`self.ApplyProperties`)
  ;[1 1 1] Sets Terrain Detection for Dust VFX
  (`KismetSystemLibrary.K2_SetTimer` null "DetectTerrain" 0.1 true)
  ;[1 1 1] Gets Initial information from JSBSim for Gears and Flaps
  (set `self.Commands` (`/Game/VigilanteMovement/Shared/Blueprints/Base/AirVehicles/Common/BP_AirVehicle_JSBSim.Commands` _jsbsimmovement))
  (set `self.Gear Down` (`.GearDown` (break `` (`/Game/VigilanteMovement/Shared/Blueprints/Base/AirVehicles/Common/BP_AirVehicle_JSBSim.Commands` _jsbsimmovement))))
  (set `self.FlapPosition` (`/Game/VigilanteMovement/Shared/Blueprints/Base/AirVehicles/Common/BP_AirVehicle_JSBSim.FlapPositionAtStart` _jsbsimmovement))
  (for (_ _array_index) (`/Game/VigilanteMovement/Shared/Blueprints/Base/AirVehicles/Common/BP_AirVehicle_JSBSim.EngineCommands` _jsbsimmovement)
    _))

(event `SetYaw`
  (params (YawValue :type "Float (double-precision)"))
  ;[1 1 1] Events used by Child BP
)

(event `SetRoll`
  (params (RollValue :type "Float (double-precision)"))
  ;[1 1 1] Events used by Child BP
)

(event `self.ReceiveTick`
  (params (DeltaSeconds :type "Float (single-precision)"))
  ;[1 1 1] Updates JSBSim Properties, Commands and States of AirVehicle
  (`parent.ReceiveTick` DeltaSeconds)
  (`self.ApplyProperties`)
  (`self.ApplyFlightCommands`)
  (`self.UpdateGearsNormalValue`)
  (`self.UpdateFlyData`)
  (`self.UpdateEnginesRPM`)
  (if (`/Game/VigilanteMovement/Shared/Blueprints/Base/AirVehicles/Common/BP_AirVehicle_JSBSim.DrawDebug` (`self.JSBSimMovement`))
    (`self.PrintAircraftProperties`)))

(event `InputAxis|Thrust`
  (params (AxisValue :type "Float (single-precision)"))
  (set `self.Throttle` AxisValue))

(event `InputAction|TrimYawUp`
  (params (Key :type "Key Structure"))
  (:`Pressed`
    (set `self.YawTrim` (+ (`self.YawTrim`) (`self.TrimStep`)))))

(event `InputAction|Gears`
  (params (Key :type "Key Structure"))
  (:`Pressed`
    (`self.ToggleGears`)))

(event `InputAxis|Roll`
  (params (AxisValue :type "Float (single-precision)"))
  (bind _output_get (set `self.AileronControl` AxisValue))
  (`self.SetRoll` _output_get))

(event `InputAction|TrimYawDown`
  (params (Key :type "Key Structure"))
  (:`Pressed`
    (set `self.YawTrim` (- (`self.YawTrim`) (`self.TrimStep`)))))

(event `InputAxis|Pitch`
  (params (AxisValue :type "Float (single-precision)"))
  (bind _output_get (set `self.ElevatorControl` AxisValue))
  (`self.SetPitch` _output_get))

(event `InputAxis|MoveRight`
  (params (AxisValue :type "Float (single-precision)"))
  (bind _output_get (set `self.RudderControl` AxisValue))
  (`self.SetYaw` _output_get))

(event `InputAction|TrimRollUp`
  (params (Key :type "Key Structure"))
  (:`Pressed`
    (set `self.RollTrim` (+ (`self.RollTrim`) (`self.TrimStep`)))))

(event `InputAxis|Spoilers`
  (params (AxisValue :type "Float (single-precision)"))
  (set `self.Spoilers` AxisValue))

(event `InputAction|Flaps`
  (params (Key :type "Key Structure"))
  (:`Pressed`
    (`self.ToggleFlaps`)))

(event `InputAction|TrimRollDown`
  (params (Key :type "Key Structure"))
  (:`Pressed`
    (set `self.RollTrim` (- (`self.RollTrim`) (`self.TrimStep`)))))

(event `InputAction|Handbrake`
  (params (Key :type "Key Structure"))
  (:`Pressed`
    (`self.ToggleAirBrake`)))

(event `InputAxis|LeftBrake`
  (params (AxisValue :type "Float (single-precision)"))
  (set `self.Left Brake` AxisValue))

(event `InputAction|TrimPitchUp`
  (params (Key :type "Key Structure"))
  (:`Pressed`
    (set `self.PitchTrim` (+ (`self.PitchTrim`) (`self.TrimStep`)))))

(event `InputAxis|RightBrake`
  (params (AxisValue :type "Float (single-precision)"))
  (set `self.Right Brake` AxisValue))

(event `InputAxis|CenterBrake`
  (params (AxisValue :type "Float (single-precision)"))
  (set `self.Center Brake` AxisValue))

(event `InputAction|TrimPitchDown`
  (params (Key :type "Key Structure"))
  (:`Pressed`
    (set `self.PitchTrim` (- (`self.PitchTrim`) (`self.TrimStep`)))))

(event `InputAxis|Steer`
  (params (AxisValue :type "Float (single-precision)"))
  (set `self.WheelSteer` AxisValue))

(event `InputAction|ParkingBrake`
  (params (Key :type "Key Structure"))
  (:`Pressed`
    (`/Engine/EditorBlueprintResources/StandardMacros.FlipFlop`
      (:`A`
        (set `self.Parking Brake` 1.0))
      (:`B`
        (set `self.Parking Brake` 0.0)))))

(event `InputAction|ResetTrim`
  (params (Key :type "Key Structure"))
  (:`Pressed`
    (set `self.RollTrim` 0.0)
    (set `self.PitchTrim` 0.0)
    (set `self.YawTrim` 0.0)))

(fn `ApplyFlightCommands`
  ;[1 1 1] Flight navigation and trimming system are applied at this stage, most of the aircrafts will deal with this systems.
)

(fn `ApplyProperties`
  (bind _jsbsimmovement (`self.JSBSimMovement`))
  ;[1 1 1] Applies Properties for JSBSim
  (`self.SetBatchCommandsPropertyDouble` _jsbsimmovement (`self.DoubleProperties`))
  (`self.SetBatchCommandsPropertyString` _jsbsimmovement (`self.StringProperties`)))

(fn `DetectTerrain`
  (bind _returnvalue (`self.K2_GetActorLocation`))
  ;[1 1 1] Detects Terrain and Obstacles to spawn Dust Whirl VFX
  (bind (_outhits _returnvalue_2) (`KismetSystemLibrary.SphereTraceMulti` _returnvalue (+ _returnvalue (`self.TerrainDetectionOffset`)) (`self.TerrainDetectionRadius`) "TraceTypeQuery1"))
  (if _returnvalue_2
    (set `self.ShowDust` true)
    (else
      (set `self.ShowDust` false))))

(fn `InitProjectile`
  (params (BaseProjectileMovement :type "ProjectileMovementComponent Object Reference"))
  (`parent.InitProjectile` BaseProjectileMovement)
  (set `ProjectileMovementComponent.bInitialVelocityInLocalSpace` true BaseProjectileMovement)
  (set `ProjectileMovementComponent.InitialSpeed` (* (`self.CASknts`) 55.5) BaseProjectileMovement))

(fn `PrintAircraftProperties`
  (bind _stringproperties (`self.StringProperties`))
  (bind _doubleproperties (`self.DoubleProperties`))
  ;[1 1 1] Prints JSBSim Properties on Screen for debug
  (`KismetSystemLibrary.PrintString` "---------------------Properties-----------------------" true false (struct :`G` 0.66 :`B` 1.0 :`A` 1.0) 0.0)
  (bind _keys (`BlueprintMapLibrary.Map_Keys` _doubleproperties))
  (for _array_element _keys
    (`KismetSystemLibrary.PrintString` (`KismetStringLibrary.Concat_StrStr` (`KismetStringLibrary.Conv_NameToString` _array_element) "::" (`KismetStringLibrary.Conv_DoubleToString` (`BlueprintMapLibrary.Map_Find` _doubleproperties _array_element))) true false (struct :`G` 0.66 :`B` 1.0 :`A` 1.0) 0.0))
  (bind _keys_2 (`BlueprintMapLibrary.Map_Keys` _stringproperties))
  (for _array_element_2 _keys_2
    (`KismetSystemLibrary.PrintString` (`KismetStringLibrary.Concat_StrStr` (`KismetStringLibrary.Conv_NameToString` _array_element_2) "::" (`BlueprintMapLibrary.Map_Find` _stringproperties _array_element_2)) true false (struct :`G` 0.66 :`B` 1.0 :`A` 1.0) 0.0))
  (`KismetSystemLibrary.PrintString` "---------------------------------------------------" true false (struct :`G` 0.66 :`B` 1.0 :`A` 1.0) 0.0))

(fn `ToggleAirBrake`
  (if (!= (`self.Speed Brake`) 0.0)
    (set `self.Speed Brake` 0.0)
    (else
      (set `self.Speed Brake` 1.0))))

(fn `ToggleFlaps`
  (if (!= (`self.FlapPosition`) 0.0)
    (set `self.FlapPosition` 0.0)
    (else
      (set `self.FlapPosition` 1.0))))

(fn `ToggleGears`
  (if (!= (`self.Gear Down`) 0.0)
    (set `self.Gear Down` 0.0)
    (else
      (set `self.Gear Down` 1.0))))

(fn `UpdateEnginesRPM`
  ;[1 1 1] Updates Engines RPM for ABP
  (`KismetArrayLibrary.Array_Clear` (`self.EnginesRPM`))
  (for _array_element (`/Game/VigilanteMovement/Shared/Blueprints/Base/AirVehicles/Common/BP_AirVehicle_JSBSim.EngineStates` (`self.JSBSimMovement`))
    (`KismetArrayLibrary.Array_Add` (`self.EnginesRPM`) (`.EngineRPM` (break `` _array_element)))))

(fn `UpdateFlyData`
  (bind (_calibratedairspeedkts _altitudeaslft _crashed) (break `` (`/Game/VigilanteMovement/Shared/Blueprints/Base/AirVehicles/Common/BP_AirVehicle_JSBSim.AircraftState` (`self.JSBSimMovement`))))
  ;[1 1 1] Updates Fly Data from JSBSim
  (set `self.CASknts` _calibratedairspeedkts)
  (set `self.Altitude ASLFt` _altitudeaslft)
  (bind _output_get (set `self.Crashed` _crashed))
  (if _output_get
    (`self.SetDamagedMode` true)))

(fn `UpdateGearsNormalValue`
  ;[1 1 1] Udpates Landing Gears Position for ABP
  (`KismetArrayLibrary.Array_Clear` (`self.GearNormValue`))
  (`KismetArrayLibrary.Array_Clear` (`self.WheelsVelocity`))
  (for _array_element (`/Game/VigilanteMovement/Shared/Blueprints/Base/AirVehicles/Common/BP_AirVehicle_JSBSim.Gears` (`self.JSBSimMovement`))
    (bind (_normalizedposition _wheelrolllinearvelocitymeterspersec) (break `` _array_element))
    (`KismetArrayLibrary.Array_Add` (`self.GearNormValue`) (- 1.0 _normalizedposition))
    (`KismetArrayLibrary.Array_Add` (`self.WheelsVelocity`) _wheelrolllinearvelocitymeterspersec)))

(fn `UserConstructionScript`
  (`parent.UserConstructionScript`))