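; Base missile projectile that simulates a timed rocket engine, starting at spawn or after an optional delay.
; While the engine runs, Niagara is active, gravity is off, and a looping timer nudges local forward velocity up or down toward the missile's max speed.
; When the running time ends, the engine stops: the effect deactivates, gravity returns and the acceleration timer clears.
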(event `self.ReceiveBeginPlay`
  (`parent.ReceiveBeginPlay`)
  ;[1 1 1] Starts Engine
  (if (> (`self.EngineStartDelay`) 0.0)
    (`KismetSystemLibrary.K2_SetTimer` null "StartEngine" (`self.EngineStartDelay`))
    (else
      (`self.StartEngine`))))

(fn `Accelerate`
  (locals (L_Multiply :type "Float (double-precision)"))
  (bind _returnvalue (`KismetMathLibrary.InverseTransformDirection` (`self.GetTransform`) (`MovementComponent.Velocity` (`self.ProjectileMovement`))))
  ;[1 1 1] Acceleration to Max Speed
  (if (>= (`self.MissileMaxSpeed`) (.x _returnvalue))
    (set `local.L_Multiply` 1.0)
    (else
      (set `local.L_Multiply` -1.0)))
  (`ProjectileMovementComponent.SetVelocityInLocalSpace` (`self.ProjectileMovement`) (+ (`KismetMathLibrary.MakeVector` (* (`local.L_Multiply`) (`self.AccelerateRate`))) _returnvalue)))

(fn `StartEngine`
  ;[1 1 1] Starts Engine
  (`ActorComponent.SetActive` (`self.Niagara`) true true)
  (set `ProjectileMovementComponent.ProjectileGravityScale` 0.0 (`self.ProjectileMovement`))
  (`KismetSystemLibrary.K2_SetTimer` null "Accelerate" 0.1 true)
  (`KismetSystemLibrary.K2_SetTimer` null "StopEngine" (`self.EngineRunningTime`)))

(fn `StopEngine`
  ;[1 1 1] Stops Engine
  (`ActorComponent.SetActive` (`self.Niagara`) false true)
  (set `ProjectileMovementComponent.ProjectileGravityScale` 1.0 (`self.ProjectileMovement`))
  (if (`KismetSystemLibrary.K2_IsTimerActive` null "Accelerate")
    (`KismetSystemLibrary.K2_ClearTimer` null "Accelerate")))

(fn `UserConstructionScript`
  (`parent.UserConstructionScript`))